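; Zombie enemy pawn that chases the player character and takes damage.
; Tick yaws the mesh toward the player camera and, when distance is at or beyond DetectRange, runs AIMoveTo toward the player, setting BP_AnimZombie's detected and close flags.
; EnemyApplyDmg lowers clamped 0–1 health and, at zero, destroys the actor after a delay.
; Ragdoll, health UI and item roulette functions are called but empty.
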(event Custom|EnemyApplyDmg
  (params (DamageQty :type Float%20%28single-precision%29))
  ;[1 1 1] HealthManagement
  (Variables|Default|SetCurrentHealth (Math|Float|Clamp(Float) (- (Variables|Default|GetCurrentHealth) DamageQty)))
  (CallFunction|UpdateUIHealth)
  (if (== (Math|Float|Clamp(Float) (- (Variables|Default|GetCurrentHealth) DamageQty)) 0.0)
    ;[1 1 1] OnDeath
    (CallFunction|EnableRagdoll)
    (Utilities|FlowControl|Delay 3.0)
    (CallFunction|ItemRoulette)
    (Actor|DestroyActor)))

(event EventBeginPlay)

(event Collision|EventActorBeginOverlap
  (params (OtherActor :type Actor%20Object%20Reference)))

(event EventTick
  (params (DeltaSeconds :type Float%20%28single-precision%29))
  (bind _skeletalmesh (Variables|Default|GetSkeletalMesh))
  (bind _returnvalue (Components|SkeletalMesh|GetAnimInstance _skeletalmesh))
  (CallFunction|UpdateLookPos)
  (bind _returnvalue_2 (Actor|GetActorOfClass "/Game/MyStuff/MyThirdPersonTPCharacter.MyThirdPersonTPCharacter_C"))
  (bind _output_get (Variables|Default|SetCurrentDistance (Math|Vector|VectorLength (- (Transformation|GetActorLocation _returnvalue_2) (Transformation|GetActorLocation self)))))
  (bind _output_get_2 (Variables|Default|SetisDetected (>= _output_get (Variables|Default|GetDetectRange))))
  (if _output_get_2
    (bind _aspawn (Utilities|Casting|CastToPawn self)
      (:then
        (AI|AIMoveTo _aspawn (Transformation|GetActorLocation _returnvalue_2) 0 5.0 false
          (:then
            (bind _asbp_anim_zombie (Utilities|Casting|CastToBP_AnimZombie _returnvalue))
            (Variables|/Game/Model/Enemy/BP_AnimZombie.BP_AnimZombie_C|SetParam_isDetected _asbp_anim_zombie true))
          (:OnSuccess
            (bind _asbp_anim_zombie_2 (Utilities|Casting|CastToBP_AnimZombie _returnvalue))
            (Variables|/Game/Model/Enemy/BP_AnimZombie.BP_AnimZombie_C|SetParam_isClose _asbp_anim_zombie_2 true))
          (:OnFail
            (bind _asbp_anim_zombie_3 (Utilities|Casting|CastToBP_AnimZombie _returnvalue))
            (Variables|/Game/Model/Enemy/BP_AnimZombie.BP_AnimZombie_C|SetParam_isClose _asbp_anim_zombie_3 false))))
      (:CastFailed
        (Development|PrintString "Cast to pawn fail")))
    (else
      (bind _asbp_anim_zombie_4 (Utilities|Casting|CastToBP_AnimZombie _returnvalue))
      (Variables|/Game/Model/Enemy/BP_AnimZombie.BP_AnimZombie_C|SetParam_isDetected _asbp_anim_zombie_4 false))))

(fn ConstructionScript)

(fn UpdateLookPos
  (Transformation|SetWorldRotation (Variables|Default|GetSkeletalMesh) (Math|Rotator|MakeRotator 0.0 0.0 (.Yaw (Math|Rotator|BreakRotator (Math|Rotator|FindLookatRotation (Transformation|GetWorldLocation (Variables|Default|GetSkeletalMesh)) (Camera|GetCameraLocation (Game|GetPlayerCameraManager 0)))))) false false))

(fn EnableRagdoll)

(fn UpdateUIHealth)

(fn ItemRoulette)
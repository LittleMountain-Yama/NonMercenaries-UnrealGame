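; Health pickup that heals the player character and awards points when touched.
; Overlap by a MyThirdPersonTPCharacter triggers OnContact, which calls HealPlayer with HealAmount, plays a 2D herb pickup sound and runs AddPoints to raise TotalPoints.
; Both the heal and the points target the character found by GetActorOfClass, rather than the overlapping actor.
; The pickup destroys itself after a short delay.
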(event Custom|OnContact
  (bind _returnvalue (Actor|GetActorOfClass "/Game/MyStuff/BPs/MyThirdPersonTPCharacter.MyThirdPersonTPCharacter_C"))
  (Default|HealPlayer _returnvalue (Variables|Default|GetHealAmount))
  (Audio|PlaySound2D "/Game/MyStuff/Art/RE4_-_Herb_Pickup.RE4_-_Herb_Pickup" 0.5 1.0 0.0 0 0)
  (CallFunction|AddPoints)
  (Utilities|FlowControl|Delay 0.2)
  (Actor|DestroyActor))

(event EventBeginPlay)

(event Collision|EventActorBeginOverlap
  (params (OtherActor :type Actor%20Object%20Reference))
  (Utilities|Casting|CastToMyThirdPersonTPCharacter OtherActor)
  (CallFunction|OnContact))

(event EventTick
  (params (DeltaSeconds :type Float%20%28single-precision%29)))

(fn ConstructionScript)

(fn AddPoints
  (bind _returnvalue (Actor|GetActorOfClass "/Game/MyStuff/BPs/MyThirdPersonTPCharacter.MyThirdPersonTPCharacter_C"))
  (Variables|/Game/MyStuff/BPs/MyThirdPersonTPCharacter.MyThirdPersonTPCharacter_C|SetTotalPoints _returnvalue (+ (Variables|/Game/MyStuff/BPs/MyThirdPersonTPCharacter.MyThirdPersonTPCharacter_C|GetTotalPoints _returnvalue) 100)))